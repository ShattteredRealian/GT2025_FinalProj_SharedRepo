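; Teleporters_BP is a pair of linked teleport pads that move the player to the opposite pad after standing on one for TeleportTime.
; Each pad's sphere overlap starts a timer that calls Teleport, which relocates the player and sets a shared cooldown to prevent bouncing back.
; Leaving a sphere, rechecked after a short delay, cancels the timer and clears the cooldown.
; BeginPlay tints both pads' particle effects purple.
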(event OnComponentBeginOverlap(Sphere1)
  (params (OverlappedComponent :type Primitive%20Component%20Object%20Reference) (OtherActor :type Actor%20Object%20Reference) (OtherComp :type Primitive%20Component%20Object%20Reference) (OtherBodyIndex :type Integer) (bFromSweep :type Boolean) (SweepResult :type Hit%20Result%20Structure%20%28by%20ref%29))
  (if (and (not (Variables|Default|GetOnCooldown?)) (== OtherComp (Variables|/Script/Engine.Character|GetCapsuleComponent (Game|GetPlayerCharacter 0))))
    (bind _returnvalue (Utilities|Time|SetTimerbyEvent (delegate Custom|TeleportTo2) (Variables|Default|GetTeleportTime)))
    (Variables|Default|SetTeleportTimer _returnvalue)))

(event OnComponentEndOverlap(Sphere1)
  (params (OverlappedComponent :type Primitive%20Component%20Object%20Reference) (OtherActor :type Actor%20Object%20Reference) (OtherComp :type Primitive%20Component%20Object%20Reference) (OtherBodyIndex :type Integer))
  (Utilities|FlowControl|Delay 0.1)
  (if (not (Collision|IsOverlappingActor (Variables|Default|GetSphere1) (Game|GetPlayerCharacter 0) :!class /Script/Engine.PrimitiveComponent))
    (Utilities|Time|ClearandInvalidateTimerbyHandle (Variables|Default|GetTeleportTimer))
    (Variables|Default|SetOnCooldown? false)))

(event OnComponentBeginOverlap(Sphere2)
  (params (OverlappedComponent :type Primitive%20Component%20Object%20Reference) (OtherActor :type Actor%20Object%20Reference) (OtherComp :type Primitive%20Component%20Object%20Reference) (OtherBodyIndex :type Integer) (bFromSweep :type Boolean) (SweepResult :type Hit%20Result%20Structure%20%28by%20ref%29))
  (if (and (not (Variables|Default|GetOnCooldown?)) (== OtherComp (Variables|/Script/Engine.Character|GetCapsuleComponent (Game|GetPlayerCharacter 0))))
    (bind _returnvalue (Utilities|Time|SetTimerbyEvent (delegate Custom|TeleportTo1) (Variables|Default|GetTeleportTime)))
    (Variables|Default|SetTeleportTimer _returnvalue)))

(event OnComponentEndOverlap(Sphere2)
  (params (OverlappedComponent :type Primitive%20Component%20Object%20Reference) (OtherActor :type Actor%20Object%20Reference) (OtherComp :type Primitive%20Component%20Object%20Reference) (OtherBodyIndex :type Integer))
  (Utilities|FlowControl|Delay 0.1)
  (if (not (Collision|IsOverlappingActor (Variables|Default|GetSphere2) (Game|GetPlayerCharacter 0) :!class /Script/Engine.PrimitiveComponent))
    (Utilities|Time|ClearandInvalidateTimerbyHandle (Variables|Default|GetTeleportTimer))
    (Variables|Default|SetOnCooldown? false)))

(event Custom|TeleportTo2
  (CallFunction|Teleport (Transformation|GetWorldLocation (Variables|Default|GetPadMesh2))))

(event Custom|TeleportTo1
  (CallFunction|Teleport (Transformation|GetWorldLocation (Variables|Default|GetPadMesh1))))

(event EventBeginPlay
  (Effects|Components|ParticleSystem|SetColorParameter (Variables|Default|GetPulse2) "Color" "(R=0.485150,G=0.005182,B=0.938686,A=1.000000)"))

(fn ConstructionScript)

(fn Teleport
  (params (Target :type Vector))
  (Transformation|SetActorLocation (Game|GetPlayerCharacter 0) Target false false)
  (Variables|Default|SetOnCooldown? true))