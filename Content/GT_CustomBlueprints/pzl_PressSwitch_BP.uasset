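; Puzzle pressure switch that activates a linked door while an actor tagged "Heavy" rests on it.
; Begin overlap calls SwitchActivated on DoorToActivate, swaps to the on material, plays a sound and lowers or raises the switch via a timeline.
; End overlap rechecks remaining overlaps and only deactivates the door, restores the material and reverses the timeline when no Heavy actor remains.
; Both sounds play at world origin rather than at the switch.
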(event Collision|EventActorBeginOverlap
  (params (OtherActor :type Actor%20Object%20Reference))
  (if (Actor|ActorHasTag OtherActor "Heavy")
    (Development|PrintString "Feeling It!")
    (if (not (Variables|Default|GetIsPressed?))
      (Variables|Default|SetIsPressed? true)
      (Default|SwitchActivated (Variables|Default|GetDoorToActivate))
      (Rendering|Material|SetMaterial (Variables|Default|GetSwitch) 0 "/Game/Unsorted/switch_on.switch_on")
      (Audio|PlaySoundatLocation "/Game/StarterContent/Audio/Collapse01.Collapse01" "0, 0, 0" "0, 0, 0" 1.0 1.0 0.0 0 0 0 0)
      (bind _newtrack_0 (Timeline|Switch%20Activate Play)
        (:Update
          (Transformation|SetRelativeLocation (Variables|Default|GetSwitch) (Math|Vector|MakeVector 0.0 0.0 _newtrack_0) false false))))))

(event Collision|EventActorEndOverlap
  (params (OtherActor :type Actor%20Object%20Reference))
  (Variables|Default|SetWeighted? false)
  (for _array_element (Collision|GetOverlappingActors 0 :!class /Script/Engine.Actor)
    (if (Actor|ActorHasTag _array_element "Heavy")
      (Variables|Default|SetWeighted? true)))
  (if (not (Variables|Default|GetWeighted?))
    (if (not (not (Variables|Default|GetIsPressed?)))
      (Variables|Default|SetIsPressed? false)
      (Default|SwitchDeactivated (Variables|Default|GetDoorToActivate))
      (Rendering|Material|SetMaterial (Variables|Default|GetSwitch) 0 "/Game/Unsorted/switch_off.switch_off")
      (Audio|PlaySoundatLocation "/Game/SmallSoundKit/SSKCue/DoorsCue/Drs_Chest_Open_01_Cue.Drs_Chest_Open_01_Cue" "0, 0, 0" "0, 0, 0" 1.0 1.0 0.0 0 0 0 0)
      (bind _newtrack_0 (Timeline|Switch%20Activate Reverse)
        (:Update
          (Transformation|SetRelativeLocation (Variables|Default|GetSwitch) (Math|Vector|MakeVector 0.0 0.0 _newtrack_0) false false))))))

(fn ConstructionScript)