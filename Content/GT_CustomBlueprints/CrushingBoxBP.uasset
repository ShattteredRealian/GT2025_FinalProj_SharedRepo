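; CrushingBoxBP is a crusher hazard meant to move a box and heavily damage the player it presses against.
; Overlap events track player contact, and BeginPlay calls Crush after a start delay, but Crush is empty.
; The disconnected Movement timeline holds the swept cube motion, damage on a blocking hit while overlapping, and delayed restart loop.
; A tag-based damage branch is also unreachable, so the box neither moves nor deals damage as wired.
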(event OnComponentBeginOverlap(Cube)
  (params (OverlappedComponent :type Primitive%20Component%20Object%20Reference) (OtherActor :type Actor%20Object%20Reference) (OtherComp :type Primitive%20Component%20Object%20Reference) (OtherBodyIndex :type Integer) (bFromSweep :type Boolean) (SweepResult :type Hit%20Result%20Structure%20%28by%20ref%29))
  ;[0.15 0.15 0.15 0.5] Touch Test
  (Utilities|Casting|CastToBP_ThirdPersonCharacter OtherActor)
  (Variables|Default|SetIsOverlapping? true))

(event Custom|Crush
  ;[0.15 0.15 0.15 0.5] Move, and then kill if it's the player
)

(event EventBeginPlay
  ;[0.15 0.15 0.15 0.5] Delay
  (Utilities|FlowControl|Delay (Variables|Default|GetStartDelay))
  (CallFunction|Crush))

(event Collision|EventActorEndOverlap
  (params (OtherActor :type Actor%20Object%20Reference))
  ;[0.15 0.15 0.15 0.5] Touch Test
  (Utilities|Casting|CastToBP_ThirdPersonCharacter OtherActor)
  (Variables|Default|SetIsOverlapping? false))

(fn ConstructionScript)