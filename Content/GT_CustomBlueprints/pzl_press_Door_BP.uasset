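; A puzzle door that swings open once enough pressure switches are active at the same time.
; Switch activation and deactivation events adjust an active count, then play or reverse the door timeline depending on whether the required count is met.
; The timeline drives the door's relative yaw through a quarter turn, and its event track plays an open or close sound at the door based on playback direction.
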(event Custom|Switch%20Activated
  (bind _door (Variables|Default|GetDoor))
  (bind _returnvalue (Transformation|GetWorldLocation _door))
  (Math|Integer|IncrementInt (Variables|Default|GetPressureSwitchesActive)
    (:%20%20
      (if (>= (Variables|Default|GetPressureSwitchesActive) (Variables|Default|GetPressureSwitchesNeeded))
        (bind (_direction _doormove) (Timeline|DoorTimeline Play)
          (:Update
            (Transformation|SetRelativeRotation (Variables|Default|GetDoor) (Math|Rotator|MakeRotator 0.0 0.0 (* _doormove 9e+01)) false false))
          (:DoorSound
            (switch Utilities|FlowControl|Switch|SwitchonETimelineDirection _direction
              (:Forward
                (Audio|PlaySoundatLocation "/Game/SmallSoundKit/SSKWav/DoorsWav/Drs_Wood_Door_Open_01.Drs_Wood_Door_Open_01" _returnvalue "0, 0, 0" 1.0 1.0 0.0 0 0 0 0))
              (:Backward
                (Audio|PlaySoundatLocation "/Game/SmallSoundKit/SSKWav/DoorsWav/Drs_Wood_DoubleDoor_Close_01.Drs_Wood_DoubleDoor_Close_01" _returnvalue "0, 0, 0" 1.0 1.0 0.0 0 0 0 0)))))
        (else
          (Timeline|DoorTimeline Reverse))))))

(event Custom|Switch%20Deactivated
  (bind _door (Variables|Default|GetDoor))
  (bind _returnvalue (Transformation|GetWorldLocation _door))
  (Math|Integer|DecrementInt (Variables|Default|GetPressureSwitchesActive)
    (:%20%20
      (if (>= (Variables|Default|GetPressureSwitchesActive) (Variables|Default|GetPressureSwitchesNeeded))
        (bind (_direction _doormove) (Timeline|DoorTimeline Play)
          (:Update
            (Transformation|SetRelativeRotation (Variables|Default|GetDoor) (Math|Rotator|MakeRotator 0.0 0.0 (* _doormove 9e+01)) false false))
          (:DoorSound
            (switch Utilities|FlowControl|Switch|SwitchonETimelineDirection _direction
              (:Forward
                (Audio|PlaySoundatLocation "/Game/SmallSoundKit/SSKWav/DoorsWav/Drs_Wood_Door_Open_01.Drs_Wood_Door_Open_01" _returnvalue "0, 0, 0" 1.0 1.0 0.0 0 0 0 0))
              (:Backward
                (Audio|PlaySoundatLocation "/Game/SmallSoundKit/SSKWav/DoorsWav/Drs_Wood_DoubleDoor_Close_01.Drs_Wood_DoubleDoor_Close_01" _returnvalue "0, 0, 0" 1.0 1.0 0.0 0 0 0 0)))))
        (else
          (Timeline|DoorTimeline Reverse))))))

(fn ConstructionScript)